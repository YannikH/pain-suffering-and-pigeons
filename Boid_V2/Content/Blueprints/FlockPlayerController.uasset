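; Player controller for a flocking game mode that puts a tuning UI for the flock on screen.
; On BeginPlay it prints a startup message, then creates a FlockConfigurator widget and adds it to the viewport.
; Every Tick it polls the widget's cohesion, alignment and separation values and copies them into its own variables.
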(event `self.ReceiveBeginPlay`
  (`KismetSystemLibrary.PrintString` "Starting gamemode")
  (bind _returnvalue (`|CreateWidget` "/Game/UI/FlockConfigurator.FlockConfigurator_C" self))
  (`UserWidget.AddToViewport` _returnvalue 0))

(event `self.ReceiveTick`
  (params (DeltaSeconds :type "Float (single-precision)"))
  (set `self.pc_coherence` (`/Game/UI/FlockConfigurator.Cohesion` (stale `self.ReceiveBeginPlay` _returnvalue)))
  (set `self.pc_align` (`/Game/UI/FlockConfigurator.Alignment` (stale `self.ReceiveBeginPlay` _returnvalue)))
  (set `self.pc_sep` (`/Game/UI/FlockConfigurator.Separation` (stale `self.ReceiveBeginPlay` _returnvalue))))

(fn `UserConstructionScript`)